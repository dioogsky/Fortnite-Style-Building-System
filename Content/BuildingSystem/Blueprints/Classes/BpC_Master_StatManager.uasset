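; Base stat manager, apparently a component, storing integer stats in a map from stat type to min, current and max values.
; SetStat clamps new values to each stat's range, ignoring missing keys and the first enum entry, while ModifyStat applies non-zero deltas through it.
; UpdateStat and OnStatsSetUp are empty hooks, presumably for children.
; SetUpStats removes one entry and fires OnStatsSetUp, but its per-stat initialization is disconnected.
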(event `SetUpStats`
  (bind _stats (`self.Stats`))
  (`BlueprintMapLibrary.Map_Remove` _stats)
  (bind _keys (`BlueprintMapLibrary.Map_Keys` _stats))
  (for _array_element _keys
    _)
  (`self.OnStatsSetUp`))

(event `OnStatsSetUp`)

(fn `GetStat`
  (params (Stat :type "/Game/BuildingSystem/Blueprints/enums/e_Stats Enum" :default "NewEnumerator0"))
  (returns (CurrentValue :type Integer) (StatValue :type "/Game/BuildingSystem/Blueprints/Structures/s_StateValue Structure"))
  (bind _value (`BlueprintMapLibrary.Map_Find` (`self.Stats`) Stat))
  (return (`.CurrentValue_4_604B451D44B6BE75102221A438369FD3` (break `/Game/BuildingSystem/Blueprints/Structures/s_StateValue` _value)) _value))

(fn `ModifyStat`
  (params (Stat :type "/Game/BuildingSystem/Blueprints/enums/e_Stats Enum" :default "NewEnumerator0") (by :type Integer))
  (if (!= by 0)
    (`self.SetStat` Stat (+ (`self.GetStat` Stat) by))
    (return)
    (else
      (return))))

(fn `SetStat`
  (params (Stat :type "/Game/BuildingSystem/Blueprints/enums/e_Stats Enum" :default "NewEnumerator0") (NewValue :type Integer) (`Update?` :type Boolean :default true))
  (locals (localStat :type "/Game/BuildingSystem/Blueprints/enums/e_Stats Enum" :default "NewEnumerator0"))
  (bind (_minvalue _currentvalue _maxvalue) (break `/Game/BuildingSystem/Blueprints/Structures/s_StateValue` (`.StatValue` (`self.GetStat` (`local.localStat`)))))
  (set `local.localStat` Stat)
  (bind _keys (`BlueprintMapLibrary.Map_Keys` (`self.Stats`)))
  (if (and (`KismetArrayLibrary.Array_Contains` _keys (`local.localStat`)) (`|EnumInequality` Stat "NewEnumerator0"))
    (`BlueprintMapLibrary.Map_Add` (`self.Stats`) (`local.localStat`) (make `/Game/BuildingSystem/Blueprints/Structures/s_StateValue` _minvalue (`KismetMathLibrary.Clamp` NewValue _minvalue _maxvalue) _maxvalue))
    (if `Update?`
      (`self.UpdateStat` (`local.localStat`)))
    (return)
    (else
      (return))))

(fn `UpdateStat`
  (params (Stats :type "/Game/BuildingSystem/Blueprints/enums/e_Stats Enum" :default "NewEnumerator0")))